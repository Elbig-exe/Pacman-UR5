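; FantomBlue_BP is the blue ghost enemy in a Pac-Man style game, which the player can kill for points.
; When its sphere hits a Pacman_BP in the fear state, a living ghost adds to that Pacman's score, marks itself dead and swaps to a dead mesh.
; After a short delay it repositions, keeping only its current X and Y.
; UpdateSpeed sets the FloatingPawnMovement max speed.
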(event `self.Sphere.OnComponentHit`
  (params (HitComponent :type "PrimitiveComponent Object Reference") (OtherActor :type "Actor Object Reference") (OtherComp :type "PrimitiveComponent Object Reference") (NormalImpulse :type "Vector Structure") (Hit :type "HitResult Structure (by ref)"))
  (bind _aspacman_bp (cast `/Game/Blueprints/Pacman_BP` OtherActor))
  (if (`PacmanPawn.IsFear` _aspacman_bp)
    (if (not (`self.IsDead`))
      (set `PacmanPawn.Score` (+ (`PacmanPawn.Score` _aspacman_bp) 30.0) _aspacman_bp)
      (set `self.IsDead` true)
      (`StaticMeshComponent.SetStaticMesh` (`self.Sphere`) "/Game/Pacman/Meshes/SM_Enemy_Dead.SM_Enemy_Dead")
      (`KismetSystemLibrary.Delay` 1.0)
      (`self.K2_SetActorLocation` (`KismetMathLibrary.MakeVector` (.x (`self.K2_GetActorLocation`)) (.y (`self.K2_GetActorLocation`)))))))

(fn `UpdateSpeed`
  (params (NewSpeed :type "Float (double-precision)"))
  (locals (`AI Controller` :type "AIController Object Reference"))
  (set `FloatingPawnMovement.MaxSpeed` NewSpeed (`self.FloatingPawnMovement`)))

(fn `UserConstructionScript`)